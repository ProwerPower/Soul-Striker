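; Spirit orb actor: a physics ball that slows over time and ignores the first KnightOfLight found when moving.
; A looping BeginPlay timer runs Ball Deceleration, cutting X/Y velocity by Deceleration and zeroing it near rest.
; Destructible and non-destructible bounce functions currently match, restoring each axis's stored original speed in the new direction and printing X.
; Their speed-banded multiplier chains are disconnected, and the shared Ball Bounce Function is an unfinished stub.
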(event EventBeginPlay
  ;[1 1 1] Constant ball deceleration and disable collision with players
  (bind _outactors (Actor|GetAllActorsOfClass "/Game/ThirdPersonBP/Blueprints/KnightOfLight.KnightOfLight_C"))
  (Collision|IgnoreActorwhenMoving (Variables|Default|GetSphere) (Utilities|Array|Get(acopy) _outactors) true)
  (Utilities|Time|SetTimerbyFunctionName 0 "Ball Deceleration" 0.1 true))

(fn ConstructionScript)

(fn BallBounceDestructible
  ;[1 1 1] After running through function, determine which multipler to use to determine Post Bounce Velocity
  (bind _returnvalue (Physics|GetPhysicsLinearVelocity (Variables|Default|GetSphere) "None"))
  (bind _output_get (Variables|FunctionVariables|SetNew%20Velocity%20X (.x _returnvalue)))
  (bind _output_get_2 (Variables|FunctionVariables|SetNew%20Velocity%20Y (.y _returnvalue)))
  (Variables|FunctionVariables|SetPLV%20X (* (/ (Math|Float|Absolute(Float) (Variables|FunctionVariables|GetOriginal%20Velocity%20X)) (Math|Float|Absolute(Float) (Variables|FunctionVariables|GetNew%20Velocity%20X))) _output_get))
  (Variables|FunctionVariables|SetPLV%20Y (* (/ (Math|Float|Absolute(Float) (Variables|FunctionVariables|GetOriginal%20Velocity%20Y)) (Math|Float|Absolute(Float) (Variables|FunctionVariables|GetNew%20Velocity%20Y))) _output_get_2))
  (Physics|SetPhysicsLinearVelocity (Variables|Default|GetSphere) (Math|Vector|MakeVector (Variables|FunctionVariables|GetPLV%20X) (Variables|FunctionVariables|GetPLV%20Y) 0.0) false "None")
  (Development|PrintString (Utilities|String|ToString(Float) (Variables|FunctionVariables|GetPLV%20X)) true true "(R=1.000000,G=0.006920,B=0.000000,A=1.000000)" 2.0))

(fn BallBounceNon-Destructible
  ;[1 1 1] After running through function, determine which multipler to use to determine Post Bounce Velocity
  (bind _returnvalue (Physics|GetPhysicsLinearVelocity (Variables|Default|GetSphere) "None"))
  (bind _output_get (Variables|FunctionVariables|SetNew%20Velocity%20X (.x _returnvalue)))
  (bind _output_get_2 (Variables|FunctionVariables|SetNew%20Velocity%20Y (.y _returnvalue)))
  (Variables|FunctionVariables|SetPLV%20X (* (/ (Math|Float|Absolute(Float) (Variables|FunctionVariables|GetOriginal%20Velocity%20X)) (Math|Float|Absolute(Float) (Variables|FunctionVariables|GetNew%20Velocity%20X))) _output_get))
  (Variables|FunctionVariables|SetPLV%20Y (* (/ (Math|Float|Absolute(Float) (Variables|FunctionVariables|GetOriginal%20Velocity%20Y)) (Math|Float|Absolute(Float) (Variables|FunctionVariables|GetNew%20Velocity%20Y))) _output_get_2))
  (Physics|SetPhysicsLinearVelocity (Variables|Default|GetSphere) (Math|Vector|MakeVector (Variables|FunctionVariables|GetPLV%20X) (Variables|FunctionVariables|GetPLV%20Y) 0.0) false "None")
  (Development|PrintString (Utilities|String|ToString(Float) (Variables|FunctionVariables|GetPLV%20X)) true true "(R=1.000000,G=0.006920,B=0.000000,A=1.000000)" 2.0))

(fn BallDeceleration
  (bind _returnvalue (Physics|GetPhysicsLinearVelocity (Variables|Default|GetSphere) "None"))
  (if (and (<= (.x _returnvalue) 25.0) (>= (.x _returnvalue) -25.0))
    (if (and (<= (.y _returnvalue) 25.0) (>= (.y _returnvalue) -25.0))
      (Variables|FunctionVariables|SetPLV%20Y 0.0)
      (Variables|FunctionVariables|SetPLV%20X 0.0)
      (Physics|SetPhysicsLinearVelocity (Variables|Default|GetSphere) (Math|Vector|MakeVector (Variables|FunctionVariables|GetPLV%20X) (Variables|FunctionVariables|GetPLV%20Y) 0.0) false "None")
      (else
        (bind _output_get (Variables|FunctionVariables|SetNew%20Velocity%20Y (.y _returnvalue)))
        (Variables|FunctionVariables|SetPLV%20Y (* (/ (- (Math|Float|Absolute(Float) _output_get) (Variables|FunctionVariables|GetDeceleration)) (Math|Float|Absolute(Float) _output_get)) _output_get))
        (Variables|FunctionVariables|SetPLV%20X 0.0)
        (Physics|SetPhysicsLinearVelocity (Variables|Default|GetSphere) (Math|Vector|MakeVector (Variables|FunctionVariables|GetPLV%20X) (Variables|FunctionVariables|GetPLV%20Y) 0.0) false "None")))
    (else
      (bind _output_get_2 (Variables|FunctionVariables|SetNew%20Velocity%20X (.x _returnvalue)))
      (bind _output_get_3 (Variables|FunctionVariables|SetNew%20Velocity%20Y (.y _returnvalue)))
      (Variables|FunctionVariables|SetPLV%20X (* (/ (- (Math|Float|Absolute(Float) _output_get_2) (Variables|FunctionVariables|GetDeceleration)) (Math|Float|Absolute(Float) _output_get_2)) _output_get_2))
      (Variables|FunctionVariables|SetPLV%20Y (* (/ (- (Math|Float|Absolute(Float) _output_get_3) (Variables|FunctionVariables|GetDeceleration)) (Math|Float|Absolute(Float) _output_get_3)) _output_get_3))
      (Physics|SetPhysicsLinearVelocity (Variables|Default|GetSphere) (Math|Vector|MakeVector (Variables|FunctionVariables|GetPLV%20X) (Variables|FunctionVariables|GetPLV%20Y) 0.0) false "None"))))