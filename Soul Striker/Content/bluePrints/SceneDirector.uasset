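; SceneDirector is a shared camera actor that both local players view, set up for two KnightOfLight characters.
; On BeginPlay it becomes the view target for player controllers 0 and 1 and stores both knights as P1 and P2.
; Unconnected logic would center it between them, scale camera arm length with their separation and clamp that separation.
; Tick is empty, so none of that tracking runs.
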(event EventBeginPlay
  ;[1 1 1] Make all characters use the camera component of SceneDirector
  (Game|Player|SetViewTargetwithBlend (Game|GetPlayerController 0) self 0.0 "VTBlend_Linear" 0.0 false)
  ;[1 1 1] Store References to both characters in variables
  (bind _outactors (Actor|GetAllActorsOfClass "/Game/ThirdPersonBP/Blueprints/KnightOfLight.KnightOfLight_C"))
  (Variables|Default|SetP1 (Utilities|Array|Get(acopy) _outactors))
  (Variables|Default|SetP2 (Utilities|Array|Get(acopy) _outactors 1)))

(event EventTick
  (params (DeltaSeconds :type Float%20%28single-precision%29)))

(fn ConstructionScript)