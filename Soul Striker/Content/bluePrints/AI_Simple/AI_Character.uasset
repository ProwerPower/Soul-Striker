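; AI_Character is a simple enemy AI that roams, patrols or chases based on its AIState at BeginPlay.
; Roaming loops through random nearby navigable points, while Patrol alternates two delayed AIMoveTo calls with no destinations set.
; When PawnSensing sees a KnightOfLight, ChasePlayer moves to it, applies damage on arrival and repeats after a delay.
; Behaviour runs on recursive events rather than a behavior tree.
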(event OnSeePawn(PawnSensing)
  (params (Pawn :type Pawn%20Object%20Reference))
  ;[1 1 1] Chase Player When Seen
  (bind _asknight_of_light (Utilities|Casting|CastToKnightOfLight Pawn))
  (CallFunction|ChasePlayer _asknight_of_light))

(event Custom|ChasePlayer
  (params (PlayerToChase :type Pawn%20Object%20Reference))
  ;[1 1 1] AI Chase Player
  (AI|AIMoveTo self "0, 0, 0" PlayerToChase 5.0 false
    (:OnSuccess
      (Game|Damage|ApplyDamage PlayerToChase (Variables|Default|GetDamage) 0 0)
      (Utilities|FlowControl|Delay 4.0)
      (CallFunction|ChasePlayer PlayerToChase))))

(event Custom|Roaming
  ;[1 1 1] AI Roaming
  (AI|AIMoveTo self (Class|NavigationSystem|GetRandomPointinNavigableRadius (Transformation|GetActorLocation) 5e+02) 0 5.0 false
    (:OnSuccess
      (Utilities|FlowControl|Delay 0.2)
      (CallFunction|Roaming))))

(event Custom|Patrol
  ;[1 1 1] AI Patrol
  (AI|AIMoveTo self "0, 0, 0" 0 5.0 false
    (:OnSuccess
      (Utilities|FlowControl|Delay 3.0)
      (AI|AIMoveTo self "0, 0, 0" 0 5.0 false
        (:OnSuccess
          (Utilities|FlowControl|Delay 3.0)
          (CallFunction|Patrol))))))

(event EventBeginPlay
  ;[1 1 1] Begin AI Functions
  (switch Utilities|FlowControl|Switch|SwitchonAI_State (Variables|Default|GetAIState)
    (:NewEnumerator1
      (CallFunction|Roaming))
    (:NewEnumerator2
      (CallFunction|ChasePlayer))
    (:NewEnumerator3
      (CallFunction|Patrol))))

(fn ConstructionScript)