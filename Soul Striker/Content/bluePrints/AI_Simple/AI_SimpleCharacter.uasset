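; Simple AI enemy character that roams, chases or patrols and melee-attacks the player.
; BeginPlay picks looping AIMoveTo behavior from AIState; PawnSensing starts a chase on seeing a KnightOfLight, though Patrol moves have no destination set.
; A delayed Tick check damages player 0 within range, then a counter loop restores the Attack flag.
; Incoming damage lowers Health, destroying the actor only when it equals exactly zero.
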(event OnSeePawn(PawnSensing)
  (params (Pawn :type Pawn%20Object%20Reference))
  ;[1 1 1] Chase Player When Seen
  (bind _asknight_of_light (Utilities|Casting|CastToKnightOfLight Pawn))
  (CallFunction|ChasePlayer _asknight_of_light))

(event Custom|ChasePlayer
  (params (PlayerToChase :type Pawn%20Object%20Reference))
  ;[1 1 1] AI Chase Player
  (AI|AIMoveTo self "0, 0, 0" PlayerToChase 5.0 false))

(event Custom|Roaming
  ;[1 1 1] AI Roaming
  (AI|AIMoveTo self (Class|NavigationSystem|GetRandomPointinNavigableRadius (Transformation|GetActorLocation) 5e+02) 0 5.0 false
    (:OnSuccess
      (Utilities|FlowControl|Delay 0.2)
      (CallFunction|Roaming))))

(event Custom|Patrol
  ;[1 1 1] AI Patrol
  (AI|AIMoveTo self "0, 0, 0" 0 5.0 false
    (:OnSuccess
      (Utilities|FlowControl|Delay 3.0)
      (AI|AIMoveTo self "0, 0, 0" 0 5.0 false
        (:OnSuccess
          (Utilities|FlowControl|Delay 3.0)
          (CallFunction|Patrol))))))

(event Custom|AttackDelaySet
  ;[1 1 1] Reset Attack Delay
  (while (< (Variables|Default|GetAttackDelay) 6.0)
    (Math|Float|IncrementFloat (Variables|Default|GetAttackDelay)
      (:%20%20
        (Utilities|FlowControl|Delay 1.0))))
  (Variables|Default|SetAttack? true)
  (Variables|Default|SetAttackDelay 0.0))

(event EventBeginPlay
  ;[1 1 1] Begin AI Functions
  (switch Utilities|FlowControl|Switch|SwitchonAI_State (Variables|Default|GetAIState)
    (:NewEnumerator1
      (CallFunction|Roaming))
    (:NewEnumerator2
      (CallFunction|ChasePlayer))
    (:NewEnumerator3
      (CallFunction|Patrol))))

(event Game|Damage|EventAnyDamage
  (params (Damage :type Float%20%28single-precision%29) (DamageType :type Damage%20Type%20Object%20Reference) (InstigatedBy :type Controller%20Object%20Reference) (DamageCauser :type Actor%20Object%20Reference))
  ;[1 1 1] Take Damage and Check for Death
  (Variables|Default|SetHealth (- (Variables|Default|GetHealth) Damage))
  (if (== (Variables|Default|GetHealth) 0.0)
    (Actor|DestroyActor)))

(event EventTick
  (params (DeltaSeconds :type Float%20%28single-precision%29))
  (bind _returnvalue (Game|GetPlayerCharacter 0))
  ;[1 1 1] Attack
  (Utilities|FlowControl|Delay 1.0)
  (if (Variables|Default|GetAttack?)
    (if (< (Transformation|GetDistanceTo _returnvalue) 1.5e+02)
      (Game|Damage|ApplyDamage _returnvalue (Variables|Default|GetDamage) 0 0)
      (Variables|Default|SetAttack? false)
      (CallFunction|AttackDelaySet))))

(fn ConstructionScript)